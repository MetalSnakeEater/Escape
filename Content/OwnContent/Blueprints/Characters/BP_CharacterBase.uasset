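; Base character Blueprint that plays walking and running footstep audio based on movement.
; Every Tick, it treats the character as moving when velocity is non-zero with no vertical component, and stops the sound otherwise.
; Running plays a single sound from a start offset, while walking picks a random step sound whenever the previous one ends.
; Changing between walking and running to match IsRunning swaps the sound on the shared FootstepSound component.
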(event EventBeginPlay)

(event Collision|EventActorBeginOverlap
  (params (OtherActor :type Actor%20Object%20Reference)))

(event EventTick
  (params (DeltaSeconds :type Float%20%28single-precision%29))
  (bind _footstepsound (Variables|Default|GetFootstepSound))
  (bind _footstepsound_2 (Variables|Default|GetFootstepSound))
  (bind _bmoving (CallFunction|IsCharacterMoving))
  (if _bmoving
    (if (Variables|Default|GetisRunning)
      (if (Audio|Components|Audio|IsPlaying (Variables|Default|GetFootstepSound))
        (if (not (== (Variables|/Script/Engine.AudioComponent|GetSound (Variables|Default|GetFootstepSound)) (Variables|Default|GetSoundOfRunning)))
          (Audio|Components|Audio|SetSound _footstepsound (Variables|Default|GetSoundOfRunning) :!label _label)
          (Audio|Components|Audio|Play _footstepsound 3.0))
        (else
          (goto _label)))
      (elif (Audio|Components|Audio|IsPlaying (Variables|Default|GetFootstepSound))
        (if (== (Variables|/Script/Engine.AudioComponent|GetSound (Variables|Default|GetFootstepSound)) (Variables|Default|GetSoundOfRunning))
          (Audio|Components|Audio|Stop (Variables|Default|GetFootstepSound))
          (Audio|Components|Audio|SetSound _footstepsound_2 (.OutItem (Utilities|Array|Random (Variables|Default|GetSoundsOfSteps))) :!label _label_2)
          (Audio|Components|Audio|Play _footstepsound_2 0.0))
        (else
          (goto _label_2))))
    (else
      (Audio|Components|Audio|Stop (Variables|Default|GetFootstepSound)))))

(fn ConstructionScript)

(fn IsCharacterMoving
  (bind _charactermovement (Variables|Character|GetCharacterMovement))
  (return (and (> (Math|Vector|VectorLength (Variables|/Script/Engine.MovementComponent|GetVelocity _charactermovement)) 0.0) (== (.z (Variables|/Script/Engine.MovementComponent|GetVelocity _charactermovement)) 0.0))))