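; BP_Cell_Door is a cell door actor that shows a Lock component while its IsLocked flag is set.
; BeginPlay sets the lock's visibility from the flag.
; Tick hides the lock whenever the flag is false but never shows it again, so relocking during play leaves it hidden.
; Overlap and construction only call the parent, and the file itself contains no opening or unlocking logic.
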(event EventBeginPlay
  (bind _lock (Variables|Default|GetLock))
  (|CallParentFunction)
  (if (Variables|Default|GetisLocked)
    (Rendering|SetVisibility _lock true false)
    (else
      (Rendering|SetVisibility _lock false false))))

(event Collision|EventActorBeginOverlap
  (params (OtherActor :type Actor%20Object%20Reference))
  (|CallParentFunction OtherActor))

(event EventTick
  (params (DeltaSeconds :type Float%20%28single-precision%29))
  (|CallParentFunction DeltaSeconds)
  (if (not (Variables|Default|GetisLocked))
    (Rendering|SetVisibility (Variables|Default|GetLock) false false)))

(fn ConstructionScript
  (|CallParentFunction))