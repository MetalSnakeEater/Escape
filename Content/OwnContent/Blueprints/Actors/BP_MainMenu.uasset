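; BP_MainMenu is a menu actor that hosts a BPW_Menu widget and moves the player's view between linked menu actors.
; On begin play it binds the widget's transition event and disables its own collision.
; A transition request looks up the index in LinkedMenus, swaps collision from this actor to the target, and blends the player's view target to it with an ease-out.
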(event Custom|TransitionTo
  (params (NewMenu :type BP%20Main%20Menu%20Object%20Reference))
  (Collision|SetActorEnableCollision false)
  (Collision|SetActorEnableCollision NewMenu true)
  (Game|Player|SetViewTargetwithBlend (Game|GetPlayerController 0) NewMenu 2.0 "VTBlend_EaseOut" 2.0 false))

(event Custom|OnTransitionToMenus
  (params (MenuIndex :type Integer))
  (if (Utilities|Array|IsValidIndex (Variables|Default|GetLinkedMenus) MenuIndex)
    (CallFunction|Transitionto (Utilities|Array|Get(acopy) (Variables|Default|GetLinkedMenus) MenuIndex))))

(event EventBeginPlay
  (bind _asbpw_menu (Utilities|Casting|CastToBPW_Menu (UserInterface|GetUserWidgetObject (Variables|Default|GetWidget))))
  (EventDispatchers|AssignTransitiontoLinkedMenu _asbpw_menu (delegate Custom|OnTransitionToMenus))
  (Collision|SetActorEnableCollision false))

(fn ConstructionScript)