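; BP_ExitConditionChecker is an actor that opens up an exit condition by removing a set of actors once two cubes are hidden.
; Every Tick it polls the Hidden state of the first two entries in Cubes.
; While both are hidden, it destroys each still-valid actor in ToRemove, repeating the check every frame with no one-shot guard.
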(event EventBeginPlay)

(event Collision|EventActorBeginOverlap
  (params (OtherActor :type Actor%20Object%20Reference)))

(event EventTick
  (params (DeltaSeconds :type Float%20%28single-precision%29))
  (bind _cubes (Variables|Default|GetCubes))
  (if (and (Variables|/Script/Engine.Actor|GetbHidden (Utilities|Array|Get(acopy) _cubes)) (Variables|/Script/Engine.Actor|GetbHidden (Utilities|Array|Get(acopy) _cubes 1)))
    (for _array_element (Variables|Default|GetToRemove)
      (if (Utilities|IsValid _array_element)
        (Actor|DestroyActor _array_element)))))

(fn ConstructionScript)